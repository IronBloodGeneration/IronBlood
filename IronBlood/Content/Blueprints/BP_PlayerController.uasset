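; Player controller Blueprint that moves the controlled pawn with point-and-click navigation.
; A left mouse press traces under the cursor on the Visibility channel and passes the hit to MoveCharacter.
; MoveCharacter calls SimpleMoveToLocation only when the pawn-to-hit distance lies between MinClickDistance and CharacterMoveLimit, otherwise printing a too-short or too-long message with the hit coordinates.
; A touch trace and two DoOnce nodes remain unconnected.
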(event EventBeginPlay)

(event EventTick
  (params (DeltaSeconds :type Float%20%28single-precision%29)))

(event Input|MouseEvents|LeftMouseButton
  (params (Key :type Key%20Structure :default "AnyKey"))
  (:Pressed
    (CallFunction|MoveCharacter (.HitResult (Game|Player|GetHitResultUnderCursorbyChannel (Game|GetPlayerController 0) "TraceTypeQuery1" true)))))

(fn ConstructionScript)

(fn MoveCharacter
  (params (Hit :type Hit%20Result%20Structure))
  (bind _returnvalue (Pawn|GetControlledPawn))
  (bind _location (Collision|BreakHitResult Hit))
  (bind _returnvalue_2 (Transformation|GetActorLocation _returnvalue))
  (bind (_x _y _z) (Math|Vector|BreakVector _location))
  (bind _returnvalue_3 (- _returnvalue_2 _location))
  (bind _returnvalue_4 (Utilities|String|ToString(Float) _x))
  (bind _returnvalue_5 (Utilities|String|ToString(Float) _y))
  (bind _returnvalue_6 (Utilities|String|ToString(Float) _z))
  (bind _returnvalue_7 (Math|Vector|VectorLength _returnvalue_3))
  (bind _returnvalue_8 (Utilities|String|Append _returnvalue_4 ", " _returnvalue_5 ", " _returnvalue_6))
  (if (>= _returnvalue_7 (Variables|Default|GetMinClickDistance))
    (if (<= _returnvalue_7 (Variables|Default|GetCharacterMoveLimit))
      (AI|Navigation|SimpleMovetoLocation (Game|GetPlayerController 0) _location)
      (else
        (Development|PrintString "Too long")
        (Development|PrintString _returnvalue_8)))
    (else
      (Development|PrintString "Too Short")
      (Development|PrintString _returnvalue_8))))